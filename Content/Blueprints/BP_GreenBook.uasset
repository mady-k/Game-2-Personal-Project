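; BP_GreenBook is an interactable collectible book that increments the player's item count and plays a Kiara voice line.
; Interact fires once, casts the actor from the sphere overlap to BP_ThirdPersonCharacter, increments ItemsCollected, then destroys the book.
; It also spawns BP_GreenBookTrigger at a hard-coded transform and plays the KiaraReport dialogue in 2D.
; An unconnected chain that notifies BP_LockedDoor never runs.
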(event `self.Sphere.OnComponentBeginOverlap`
  (params (OverlappedComponent :type "PrimitiveComponent Object Reference") (OtherActor :type "Actor Object Reference") (OtherComp :type "PrimitiveComponent Object Reference") (OtherBodyIndex :type Integer) (bFromSweep :type Boolean) (SweepResult :type "HitResult Structure (by ref)")))

(event `/Game/Blueprints/InteractInterface.Interact`
  (`/Engine/EditorBlueprintResources/StandardMacros.DoOnce` false
    (:`Completed`
      (`|ExecutionSequence`
        (:`then_0`
          (bind _asbp_third_person_character (cast `/Game/ThirdPerson/Blueprints/BP_ThirdPersonCharacter` (stale `self.Sphere.OnComponentBeginOverlap` OtherActor)))
          (bind _result (`/Engine/EditorBlueprintResources/StandardMacros.IncrementInt` (`/Game/ThirdPerson/Blueprints/BP_ThirdPersonCharacter.ItemsCollected` _asbp_third_person_character))
            (:`  `
              (set `/Game/ThirdPerson/Blueprints/BP_ThirdPersonCharacter.ItemsCollected` _result _asbp_third_person_character)
              (`self.K2_DestroyActor`)
              (`|SpawnActorFromClass` "/Game/Blueprints/BP_GreenBookTrigger.BP_GreenBookTrigger_C" (`KismetMathLibrary.MakeTransform` (-370.0 -1115.0 174.0) (struct) (2.15625 2.09375 1.0)) "Undefined" "MultiplyWithRoot" null null))))
        (:`then_1`
          (`GameplayStatics.PlayDialogue2D` (`self.KiaraReport`) (make `DialogueContext` (`self.KiaraVoice`) (`|MakeArray` (`self.KiaraVoice`)))))))))

(fn `UserConstructionScript`)