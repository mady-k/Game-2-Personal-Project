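; Test actor that repeatedly damages every BP_Enemy in the level, starting at BeginPlay.
; Each pass gathers the enemies with GetAllActorsOfClass, prints their count, calls TakeDamage on each with a small random amount, then prints a confirmation.
; The GiveDamage event calls itself after a short Delay, so the cycle repeats indefinitely and re-queries the enemy list every pass.
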(event `GiveDamage`
  (bind _outactors (`GameplayStatics.GetAllActorsOfClass` "/Game/Blueprints/BP_Enemy.BP_Enemy_C" :!label _label)) ; find all of the enemies in the level
  (`KismetSystemLibrary.PrintString` (`KismetStringLibrary.Concat_StrStr` "There are " (`KismetStringLibrary.Conv_IntToString` (`KismetArrayLibrary.Array_Length` _outactors)) "  enemies in the level. ") true true (struct :`G` 0.66 :`B` 1.0 :`A` 1.0) 5.0)
  (for _array_element _outactors
    (`/Game/Blueprints/BP_Enemy.TakeDamage` _array_element (`KismetMathLibrary.RandomFloatInRange` 0.1 0.5)))
  (`KismetSystemLibrary.PrintString` "We've given damage to all of the enenmies. " true true (struct :`G` 0.66 :`B` 1.0 :`A` 1.0) 5.0)
  (`KismetSystemLibrary.Delay` 2.0)
  (`self.GiveDamage`))

(event `self.ReceiveBeginPlay`
  (goto _label))

(fn `UserConstructionScript`)