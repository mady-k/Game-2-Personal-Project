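; BP_Door is an interactable door that toggles open and closed on each Interact.
; A FlipFlop plays or reverses a timeline that lerps the static mesh's yaw between 0 and 90 degrees.
; Every timeline update, in either direction, also plays a 2D hit sound and feeds a one-second Delay that then plays a Kiara dialogue line.
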(event `/Game/Blueprints/InteractInterface.Interact`
  (`/Engine/EditorBlueprintResources/StandardMacros.FlipFlop`
    (:`A`
      (bind (_direction _door_track) (`Timeline|open/Close door timeline` :!label _label)
        (:`Update`
          (`SceneComponent.K2_SetRelativeRotation` (`self.StaticMesh`) (`KismetMathLibrary.MakeRotator` 0.0 0.0 (`KismetMathLibrary.Lerp` 0.0 90.0 _door_track)) false false)
          (`GameplayStatics.PlaySound2D` "/Game/Audio/Hit_Hurt5.Hit_Hurt5" 1.0 1.0 0.0 null null)
          (`KismetSystemLibrary.Delay` 1.0)
          (`GameplayStatics.PlayDialogue2D` (`self.Kiara20`) (make `DialogueContext` (`self.KiaraVoice`) (`|MakeArray` (`self.KiaraVoice`)))))))
    (:`B`
      (goto _label :!via `Reverse`))))

(fn `UserConstructionScript`)