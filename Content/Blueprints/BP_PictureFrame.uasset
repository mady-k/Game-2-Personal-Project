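; Picture frame actor that plays two Kiara dialogue lines the first time it is interacted with.
; Interact passes a DoOnce, then casts the OtherActor from the Box overlap event to BP_ThirdPersonCharacter.
; It plays the lines as 2D dialogue separated by a short delay, the first targeting the character's voice and the second its own speaker voice.
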(event `self.Box.OnComponentBeginOverlap`
  (params (OverlappedComponent :type "PrimitiveComponent Object Reference") (OtherActor :type "Actor Object Reference") (OtherComp :type "PrimitiveComponent Object Reference") (OtherBodyIndex :type Integer) (bFromSweep :type Boolean) (SweepResult :type "HitResult Structure (by ref)")))

(event `/Game/Blueprints/InteractInterface.Interact`
  (`/Engine/EditorBlueprintResources/StandardMacros.DoOnce` false
    (:`Completed`
      (bind _asbp_third_person_character (cast `/Game/ThirdPerson/Blueprints/BP_ThirdPersonCharacter` (stale `self.Box.OnComponentBeginOverlap` OtherActor)))
      (`GameplayStatics.PlayDialogue2D` (`self.Kiara3`) (make `DialogueContext` (`self.DialogueVoice`) (`|MakeArray` (`/Game/ThirdPerson/Blueprints/BP_ThirdPersonCharacter.DialogueVoice` _asbp_third_person_character))))
      (`KismetSystemLibrary.Delay` 2.0)
      (`GameplayStatics.PlayDialogue2D` (`self.Kiara4`) (make `DialogueContext` (`self.DialogueVoice`) (`|MakeArray` (`self.DialogueVoice`)))))))

(fn `UserConstructionScript`)