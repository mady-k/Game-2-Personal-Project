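; BP_LockedDoor is a story puzzle door that swings open once the player has collected enough books.
; The first Interact plays Kiara's dialogue and spawns BP_SpeakerTrigger; every Interact checks the character's ItemsCollected before calling OpenPuzzleDoor.
; That event flip-flops a yaw timeline to open or close the door, with a dialogue exchange wired to the timeline's Update.
; The door's own item-counting logic is disconnected, leaving Collectitem without effect.
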(event `OpenPuzzleDoor`
  (`GameplayStatics.PlaySound2D` "/Game/Audio/Hit_Hurt5.Hit_Hurt5" 1.0 1.0 0.0 null null)
  (`KismetSystemLibrary.Delay` 1.0)
  (`GameplayStatics.PlayDialogue2D` (`self.Anonymous7`) (make `DialogueContext` (`self.AnonymousVoice`) (`|MakeArray` (`self.AnonymousVoice`))))
  (`/Engine/EditorBlueprintResources/StandardMacros.FlipFlop`
    (:`A`
      (bind (_direction _door_rotation) (`Timeline|open door` :!label _label)
        (:`Update`
          (`SceneComponent.K2_SetRelativeRotation` (`self.StaticMesh`) (`KismetMathLibrary.MakeRotator` 0.0 0.0 (`KismetMathLibrary.Lerp` 0.0 90.0 _door_rotation)) false false)
          (`GameplayStatics.PlayDialogue2D` (`self.Kiara17`) (make `DialogueContext` (`self.KiaraVoice`) (`|MakeArray` (`self.KiaraVoice`))))
          (`KismetSystemLibrary.Delay` 1.0)
          (`GameplayStatics.PlayDialogue2D` (`self.Anonymous8`) (make `DialogueContext` (`self.AnonymousVoice`) (`|MakeArray` (`self.AnonymousVoice`))))
          (`KismetSystemLibrary.Delay` 1.0)
          (`GameplayStatics.PlayDialogue2D` (`self.Kiara18`) (make `DialogueContext` (`self.KiaraVoice`) (`|MakeArray` (`self.KiaraVoice`))))
          (`KismetSystemLibrary.Delay` 1.0)
          (`GameplayStatics.PlayDialogue2D` (`self.Anonymous9`) (make `DialogueContext` (`self.AnonymousVoice`) (`|MakeArray` (`self.AnonymousVoice`))))
          (`KismetSystemLibrary.Delay` 1.0)
          (`GameplayStatics.PlayDialogue2D` (`self.Kiara19`) (make `DialogueContext` (`self.KiaraVoice`) (`|MakeArray` (`self.KiaraVoice`)))))))
    (:`B`
      (goto _label :!via `Reverse`))))

(event `Collectitem`
  (bind _returnvalue (`GameplayStatics.GetActorOfClass` "BP_LockedDoor_C")))

(event `OpenDoorCheck`
  (if (>= (`self.CurrentItemsCollected`) (`self.MaxItemsCollected`))
    (`/Engine/EditorBlueprintResources/StandardMacros.DoOnce` false
      (:`Completed`
        (`self.OpenPuzzleDoor`)))))

(event `/Game/Blueprints/InteractInterface.Interact`
  (`|ExecutionSequence`
    (:`then_0`
      (`/Engine/EditorBlueprintResources/StandardMacros.DoOnce` false
        (:`Completed`
          (`GameplayStatics.PlayDialogue2D` (`self.Kiara7`) (make `DialogueContext` (`self.KiaraVoice`) (`|MakeArray` (`self.KiaraVoice`))))
          (`KismetSystemLibrary.Delay` 1.0)
          (`GameplayStatics.PlaySound2D` "/Game/Audio/Hit_Hurt5.Hit_Hurt5" 1.0 1.0 0.0 null null)
          (`KismetSystemLibrary.Delay` 1.0)
          (`GameplayStatics.PlayDialogue2D` (`self.Kiara8`) (make `DialogueContext` (`self.KiaraVoice`) (`|MakeArray` (`self.KiaraVoice`))))
          (`KismetSystemLibrary.Delay` 1.0)
          (`GameplayStatics.PlaySound2D` "/Game/Audio/Hit_Hurt5.Hit_Hurt5" 1.0 1.0 0.0 null null)
          (`KismetSystemLibrary.Delay` 1.0)
          (`GameplayStatics.PlayDialogue2D` (`self.Kiara9`) (make `DialogueContext` (`self.KiaraVoice`) (`|MakeArray` (`self.KiaraVoice`))))
          (`|SpawnActorFromClass` "/Game/Blueprints/BP_SpeakerTrigger.BP_SpeakerTrigger_C" (`KismetMathLibrary.MakeTransform` (-832.0 -340.0 198.0) (struct) (2.125 3.0 6.34375)) "Undefined" "MultiplyWithRoot" null null))))
    (:`then_1`
      (bind _asbp_third_person_character (cast `/Game/ThirdPerson/Blueprints/BP_ThirdPersonCharacter` (`GameplayStatics.GetPlayerCharacter` 0)))
      (if (>= (`/Game/ThirdPerson/Blueprints/BP_ThirdPersonCharacter.ItemsCollected` _asbp_third_person_character) 4)
        (`self.OpenPuzzleDoor`)
        (else
          (`KismetSystemLibrary.PrintString` "collect more books"))))))

(fn `UserConstructionScript`)