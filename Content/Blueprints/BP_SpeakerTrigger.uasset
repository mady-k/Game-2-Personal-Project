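; Interactable speaker trigger that plays a one-time scripted conversation between Kiara and an anonymous voice.
; Interact passes a DoOnce, then casts the OtherActor from the otherwise empty box overlap event to the third-person character.
; A hard-coded chain of 2D dialogue calls alternates the two voices with fixed one-second delays.
; A hurt sound plays before Kiara's final line.
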(event `self.Box.OnComponentBeginOverlap`
  (params (OverlappedComponent :type "PrimitiveComponent Object Reference") (OtherActor :type "Actor Object Reference") (OtherComp :type "PrimitiveComponent Object Reference") (OtherBodyIndex :type Integer) (bFromSweep :type Boolean) (SweepResult :type "HitResult Structure (by ref)")))

(event `/Game/Blueprints/InteractInterface.Interact`
  (`/Engine/EditorBlueprintResources/StandardMacros.DoOnce` false
    (:`Completed`
      (cast `/Game/ThirdPerson/Blueprints/BP_ThirdPersonCharacter` (stale `self.Box.OnComponentBeginOverlap` OtherActor))
      (`GameplayStatics.PlayDialogue2D` (`self.Kiara10`) (make `DialogueContext` (`self.KiaraVoice`) (`|MakeArray` (`self.KiaraVoice`))))
      (`KismetSystemLibrary.Delay` 1.0)
      (`GameplayStatics.PlayDialogue2D` (`self.Anonymous1`) (make `DialogueContext` (`self.AnonymousVoice`) (`|MakeArray` (`self.AnonymousVoice`))))
      (`KismetSystemLibrary.Delay` 1.0)
      (`GameplayStatics.PlayDialogue2D` (`self.Kiara11`) (make `DialogueContext` (`self.KiaraVoice`) (`|MakeArray` (`self.KiaraVoice`))))
      (`KismetSystemLibrary.Delay` 1.0)
      (`GameplayStatics.PlayDialogue2D` (`self.Anonymous2`) (make `DialogueContext` (`self.AnonymousVoice`) (`|MakeArray` (`self.AnonymousVoice`))))
      (`KismetSystemLibrary.Delay` 1.0)
      (`GameplayStatics.PlayDialogue2D` (`self.Kiara12`) (make `DialogueContext` (`self.KiaraVoice`) (`|MakeArray` (`self.KiaraVoice`))))
      (`KismetSystemLibrary.Delay` 1.0)
      (`GameplayStatics.PlayDialogue2D` (`self.Anonymous3`) (make `DialogueContext` (`self.AnonymousVoice`) (`|MakeArray` (`self.AnonymousVoice`))))
      (`KismetSystemLibrary.Delay` 1.0)
      (`GameplayStatics.PlayDialogue2D` (`self.Kiara13`) (make `DialogueContext` (`self.KiaraVoice`) (`|MakeArray` (`self.KiaraVoice`))))
      (`KismetSystemLibrary.Delay` 1.0)
      (`GameplayStatics.PlayDialogue2D` (`self.Anonymous4`) (make `DialogueContext` (`self.AnonymousVoice`) (`|MakeArray` (`self.AnonymousVoice`))))
      (`KismetSystemLibrary.Delay` 1.0)
      (`GameplayStatics.PlayDialogue2D` (`self.Kiara14`) (make `DialogueContext` (`self.KiaraVoice`) (`|MakeArray` (`self.KiaraVoice`))))
      (`KismetSystemLibrary.Delay` 1.0)
      (`GameplayStatics.PlayDialogue2D` (`self.Anonymous5`) (make `DialogueContext` (`self.AnonymousVoice`) (`|MakeArray` (`self.AnonymousVoice`))))
      (`KismetSystemLibrary.Delay` 1.0)
      (`GameplayStatics.PlayDialogue2D` (`self.Kiara15`) (make `DialogueContext` (`self.KiaraVoice`) (`|MakeArray` (`self.KiaraVoice`))))
      (`KismetSystemLibrary.Delay` 1.0)
      (`GameplayStatics.PlayDialogue2D` (`self.Anonymous6`) (make `DialogueContext` (`self.AnonymousVoice`) (`|MakeArray` (`self.AnonymousVoice`))))
      (`KismetSystemLibrary.Delay` 1.0)
      (`GameplayStatics.PlaySound2D` "/Game/Audio/Hit_Hurt5.Hit_Hurt5" 1.0 1.0 0.0 null null)
      (`KismetSystemLibrary.Delay` 1.0)
      (`GameplayStatics.PlayDialogue2D` (`self.Kiara16`) (make `DialogueContext` (`self.KiaraVoice`) (`|MakeArray` (`self.KiaraVoice`)))))))

(fn `UserConstructionScript`)