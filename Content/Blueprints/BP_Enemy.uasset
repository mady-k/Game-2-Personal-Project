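; BP_Enemy is a basic enemy actor that announces itself on screen when play begins.
; A TakeDamage event prints a pain message and subtracts the given amount from Health.
; It then calls the CheckIfDead helper, which reports Health at or below zero, and destroys the actor when that is true.
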(event `self.ReceiveBeginPlay`
  (`KismetSystemLibrary.PrintString` "Hello, I have been programmed to destroy you. " true true (struct :`G` 0.66 :`B` 1.0 :`A` 1.0) 5.0))

(event `TakeDamage`
  (params (ByAmount :type "Float (double-precision)" :default 0.2))
  (`KismetSystemLibrary.PrintString` "Ouch!" true true (struct :`G` 0.66 :`B` 1.0 :`A` 1.0) 5.0)
  (bind _output_get (set `self.Health` (- (`self.Health`) ByAmount)))
  (if (`self.CheckIfDead` _output_get)
    (`self.K2_DestroyActor`)))

(fn `CheckIfDead`
  (params (Health :type "Float (double-precision)"))
  (returns (IsDead :type Boolean))
  (return (<= Health 0.0)))

(fn `UserConstructionScript`)